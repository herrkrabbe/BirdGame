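; Player controller for the bird prototype, turning Enhanced Input roll, pitch and yaw actions into pawn rotation.
; On BeginPlay it caches the player pawn as BP_BirdPrototype and adds the IMC_Bird mapping context.
; Each action converts its value to a single-axis quaternion and applies it as a local rotation delta on the bird, with no delta-time scaling.
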(event Input|EnhancedActionEvents|EnhancedInputActionIA_Pitch
  (params (ActionValue :type Float%20%28double-precision%29) (ElapsedSeconds :type Float%20%28double-precision%29) (TriggeredSeconds :type Float%20%28double-precision%29) (InputAction :type Input%20Action%20Object%20Reference :default "/Game/Input/InputAction/IA_Pitch.IA_Pitch"))
  (bind _returnvalue (Class|FlightQuaternion|EulertoQuaternion (Math|Rotator|MakeRotator 0.0 ActionValue 0.0)))
  (Class|FlightQuaternion|AddActorLocalRotationQuat (Variables|Default|GetPlayer%20Reference) _returnvalue))

(event Input|EnhancedActionEvents|EnhancedInputActionIA_Roll
  (params (ActionValue :type Float%20%28double-precision%29) (ElapsedSeconds :type Float%20%28double-precision%29) (TriggeredSeconds :type Float%20%28double-precision%29) (InputAction :type Input%20Action%20Object%20Reference :default "/Game/Input/InputAction/IA_Roll.IA_Roll"))
  (bind _returnvalue (Class|FlightQuaternion|EulertoQuaternion (Math|Rotator|MakeRotator ActionValue 0.0 0.0)))
  (Class|FlightQuaternion|AddActorLocalRotationQuat (Variables|Default|GetPlayer%20Reference) _returnvalue))

(event Input|EnhancedActionEvents|EnhancedInputActionIA_Yaw
  (params (ActionValue :type Float%20%28double-precision%29) (ElapsedSeconds :type Float%20%28double-precision%29) (TriggeredSeconds :type Float%20%28double-precision%29) (InputAction :type Input%20Action%20Object%20Reference :default "/Game/Input/InputAction/IA_Yaw.IA_Yaw"))
  (bind _returnvalue (Class|FlightQuaternion|EulertoQuaternion (Math|Rotator|MakeRotator 0.0 0.0 ActionValue)))
  (Class|FlightQuaternion|AddActorLocalRotationQuat (Variables|Default|GetPlayer%20Reference) _returnvalue))

(event EventBeginPlay
  (bind _asbp_bird_prototype (Utilities|Casting|CastToBP_BirdPrototype (Game|Player|GetPlayerPawn 0)))
  (Variables|Default|SetPlayer%20Reference _asbp_bird_prototype)
  (Input|AddMappingContext (PlayerController|LocalPlayerSubsystems|GetEnhancedInputLocalPlayerSubsystem) "/Game/Input/IMC_Bird.IMC_Bird" 0 "(bIgnoreAllPressedKeysUntilRelease=True,bForceImmediately=False,bNotifyUserSettings=False)"))

(event EventTick
  (params (DeltaSeconds :type Float%20%28single-precision%29)))

(fn ConstructionScript)