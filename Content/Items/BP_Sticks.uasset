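; BP_Sticks is a stick item that picks one of three stick meshes when play begins.
; BeginPlay runs the RandomMesh value through 1D Perlin noise to choose between SM_Stick_1 and the other two meshes.
; The split between SM_Stick_2 and SM_Stick_3 tests the raw RandomMesh value instead of the noise result.
; The file never assigns RandomMesh, and the construction script is empty.
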(event EventBeginPlay
  (if (>= (Class|KismetMathLibrary|PerlinNoise1D (Variables|Default|GetRandomMesh)) -0.33)
    (if (<= (Variables|Default|GetRandomMesh) 0.33)
      (Components|StaticMesh|SetStaticMesh (Variables|Default|GetItemMesh) "/Game/Items/SM_Stick_2.SM_Stick_2")
      (else
        (Components|StaticMesh|SetStaticMesh (Variables|Default|GetItemMesh) "/Game/Items/SM_Stick_3.SM_Stick_3")))
    (else
      (Components|StaticMesh|SetStaticMesh (Variables|Default|GetItemMesh) "/Game/Items/FBX_Files/SM_Stick_1.SM_Stick_1"))))

(event Collision|EventActorBeginOverlap
  (params (OtherActor :type Actor%20Object%20Reference)))

(event EventTick
  (params (DeltaSeconds :type Float%20%28single-precision%29)))

(fn ConstructionScript)