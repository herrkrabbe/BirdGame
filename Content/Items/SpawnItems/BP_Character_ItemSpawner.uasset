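; Wandering AI character that periodically drops random items at its own location.
; From BeginPlay it loops AI moves to random reachable nearby points, pausing briefly after each arrival and retrying on failure.
; A timer with an interval randomized once at start, looping per the Gamemode variable, calls SpawnItems.
; When SpawnEnabled, it spawns one of eight ActorsToSpawn classes and destroys it after a minute's delay.
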(event Custom|Spawn%20Items
  (if (Variables|Default|GetSpawn%20Enabled)
    (bind _returnvalue (Game|SpawnActorfromClass (Utilities|Array|Get(acopy) (Variables|Default|GetActors%20to%20Spawn) (Math|Random|RandomIntegerinRange 0 7)) (Math|Conversions|ToTransform(Vector) (Transformation|GetActorLocation)) "AdjustIfPossibleButAlwaysSpawn" "MultiplyWithRoot" 0 0))
    (Utilities|FlowControl|Delay 6e+01)
    (Actor|DestroyActor _returnvalue)))

(event Custom|Wander
  (AI|AIMoveTo self (.RandomLocation (AI|Navigation|GetRandomReachablePointinRadius (Transformation|GetActorLocation) 1e+03 0 0)) 0 1e+01 false
    (:OnSuccess
      (Utilities|FlowControl|Delay (Math|Random|RandomFloatinRange 2.0 7.0))
      (CallFunction|Wander))
    (:OnFail
      (Utilities|FlowControl|Delay 0.2)
      (CallFunction|Wander))))

(event EventBeginPlay
  (CallFunction|Wander)
  (Utilities|Time|SetTimerbyEvent (delegate Custom|Spawn%20Items) (Math|Random|RandomFloatinRange 1e+01 2.3e+02) (Variables|Default|GetGamemode)))

(event Collision|EventActorBeginOverlap
  (params (OtherActor :type Actor%20Object%20Reference)))

(event EventTick
  (params (DeltaSeconds :type Float%20%28single-precision%29)))

(fn ConstructionScript)