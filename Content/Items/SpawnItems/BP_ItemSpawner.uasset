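; BP_ItemSpawner is an actor that periodically spawns a random item at its own location.
; BeginPlay starts a timer with a single random interval of roughly 13 to 17 seconds, looping only if SpawnEnabled is set.
; Each SpawnItems call picks one of ten ActorsToSpawn indices and prints debug text.
; The printed class name uses a separate random roll, so it may differ from the spawned actor.
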(event Custom|Spawn%20Items
  (bind _returnvalue (Math|Random|RandomIntegerinRange 0 9))
  (bind _actors_to_spawn (Variables|Default|GetActors%20to%20Spawn))
  (bind _output (Utilities|Array|Get(acopy) _actors_to_spawn _returnvalue))
  (Game|SpawnActorfromClass _output (Math|Conversions|ToTransform(Vector) (Transformation|GetActorLocation)) "AdjustIfPossibleButAlwaysSpawn" "MultiplyWithRoot" 0 0)
  (Development|PrintString "Spawned Sucessfully")
  (Development|PrintString (Utilities|GetClassDisplayName _output)))

(event EventBeginPlay
  (Utilities|Time|SetTimerbyEvent (delegate Custom|Spawn%20Items) (Math|Random|RandomFloatinRange 13.0 17.0) (Variables|Default|GetSpawn%20Enabled)))

(event Collision|EventActorBeginOverlap
  (params (OtherActor :type Actor%20Object%20Reference)))

(event EventTick
  (params (DeltaSeconds :type Float%20%28single-precision%29)))

(fn ConstructionScript)