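; BP_Cup is a paper cup item that picks one of three cup meshes when play begins.
; BeginPlay runs the RandomMesh value through 1D Perlin noise, using a low result for the first mesh and otherwise the sign of RandomMesh to choose between the other two.
; The choice is applied to ItemMesh, and the file has no other active logic.
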(event EventBeginPlay
  (if (>= (Class|KismetMathLibrary|PerlinNoise1D (Variables|Default|GetRandomMesh)) -0.33)
    (if (<= (Variables|Default|GetRandomMesh) 0.0)
      (Components|StaticMesh|SetStaticMesh (Variables|Default|GetItemMesh) "/Game/Items/SM_PaperCup_2.SM_PaperCup_2")
      (else
        (Components|StaticMesh|SetStaticMesh (Variables|Default|GetItemMesh) "/Game/Items/SM_PaperCup_3.SM_PaperCup_3")))
    (else
      (Components|StaticMesh|SetStaticMesh (Variables|Default|GetItemMesh) "/Game/Items/SM_PaperCup_1.SM_PaperCup_1"))))

(event Collision|EventActorBeginOverlap
  (params (OtherActor :type Actor%20Object%20Reference)))

(event EventTick
  (params (DeltaSeconds :type Float%20%28single-precision%29)))

(fn ConstructionScript)