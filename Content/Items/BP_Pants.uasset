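; BP_Pants is an item actor that picks one of three briefs meshes for its ItemMesh on BeginPlay.
; Perlin noise of RandomMesh decides whether it gets the first mesh, while the raw RandomMesh value chooses between the other two.
; Nothing in this graph assigns RandomMesh, and the construction script is empty.
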(event EventBeginPlay
  (if (>= (Class|KismetMathLibrary|PerlinNoise1D (Variables|Default|GetRandomMesh)) -0.33)
    (if (<= (Variables|Default|GetRandomMesh) 0.33)
      (Components|StaticMesh|SetStaticMesh (Variables|Default|GetItemMesh) "/Game/Items/SM_Briefs2.SM_Briefs2")
      (else
        (Components|StaticMesh|SetStaticMesh (Variables|Default|GetItemMesh) "/Game/Items/SM_Briefs3.SM_Briefs3")))
    (else
      (Components|StaticMesh|SetStaticMesh (Variables|Default|GetItemMesh) "/Game/Items/SM_Briefs.SM_Briefs"))))

(event Collision|EventActorBeginOverlap
  (params (OtherActor :type Actor%20Object%20Reference)))

(event EventTick
  (params (DeltaSeconds :type Float%20%28single-precision%29)))

(fn ConstructionScript)