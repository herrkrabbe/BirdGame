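; BP_Card is a credit card item actor that picks one of three card meshes for its appearance.
; On BeginPlay it compares the 1D Perlin noise of RandomMesh, then RandomMesh itself, against fixed thresholds to set the static mesh on ItemMesh.
; RandomMesh is never assigned in this Blueprint's graphs, and the construction script is empty.
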(event EventBeginPlay
  (if (>= (Class|KismetMathLibrary|PerlinNoise1D (Variables|Default|GetRandomMesh)) -0.33)
    (if (<= (Variables|Default|GetRandomMesh) 0.33)
      (Components|StaticMesh|SetStaticMesh (Variables|Default|GetItemMesh) "/Game/Items/SM_CreditCard2.SM_CreditCard2")
      (else
        (Components|StaticMesh|SetStaticMesh (Variables|Default|GetItemMesh) "/Game/Items/SM_CreditCard3.SM_CreditCard3")))
    (else
      (Components|StaticMesh|SetStaticMesh (Variables|Default|GetItemMesh) "/Game/Items/SM_CreditCard.SM_CreditCard"))))

(event Collision|EventActorBeginOverlap
  (params (OtherActor :type Actor%20Object%20Reference)))

(event EventTick
  (params (DeltaSeconds :type Float%20%28single-precision%29)))

(fn ConstructionScript)