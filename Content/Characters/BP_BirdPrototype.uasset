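; Prototype bird character with flight controls driven by Enhanced Input actions for flapping, soaring and rotation.
; Flapping spends a charge that refills over time and adds an up-and-forward impulse.
; Soaring adds upward force scaled by forward speed, while pitch, roll and yaw apply local quaternion rotations to the actor.
; Nest placement, mapping-context setup and controller-rotation steering remain only as disconnected logic.
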(event Input|EnhancedActionEvents|EnhancedInputActionIA_Flap
  (params (ActionValue :type Boolean) (ElapsedSeconds :type Float%20%28double-precision%29) (TriggeredSeconds :type Float%20%28double-precision%29) (InputAction :type Input%20Action%20Object%20Reference :default "/Game/Input/InputAction/IA_Flap.IA_Flap"))
  (CallFunction|Flap)
  (Variables|Default|SetOn%20Ground false))

(event Input|EnhancedActionEvents|EnhancedInputActionIA_Pitch
  (params (ActionValue :type Float%20%28double-precision%29) (ElapsedSeconds :type Float%20%28double-precision%29) (TriggeredSeconds :type Float%20%28double-precision%29) (InputAction :type Input%20Action%20Object%20Reference :default "/Game/Input/InputAction/IA_Pitch.IA_Pitch"))
  (CallFunction|Pitch ActionValue))

(event Input|EnhancedActionEvents|EnhancedInputActionIA_Roll
  (params (ActionValue :type Boolean) (ElapsedSeconds :type Float%20%28double-precision%29) (TriggeredSeconds :type Float%20%28double-precision%29) (InputAction :type Input%20Action%20Object%20Reference :default "/Game/Input/InputAction/IA_Roll.IA_Roll"))
  (CallFunction|Roll (Math|Conversions|ToFloat(Boolean) ActionValue)))

(event Input|EnhancedActionEvents|EnhancedInputActionIA_Yaw
  (params (ActionValue :type Float%20%28double-precision%29) (ElapsedSeconds :type Float%20%28double-precision%29) (TriggeredSeconds :type Float%20%28double-precision%29) (InputAction :type Input%20Action%20Object%20Reference :default "/Game/Input/InputAction/IA_Yaw.IA_Yaw"))
  (:Triggered
    (CallFunction|Yaw ActionValue)))

(event Input|EnhancedActionEvents|EnhancedInputActionIA_Soar
  (params (ActionValue :type Boolean) (ElapsedSeconds :type Float%20%28double-precision%29) (TriggeredSeconds :type Float%20%28double-precision%29) (InputAction :type Input%20Action%20Object%20Reference :default "/Game/Input/InputAction/IA_Soar.IA_Soar"))
  (CallFunction|Lift))

(event Input|EnhancedActionEvents|EnhancedInputActionIA_Nest
  (params (ActionValue :type Boolean) (ElapsedSeconds :type Float%20%28double-precision%29) (TriggeredSeconds :type Float%20%28double-precision%29) (InputAction :type Input%20Action%20Object%20Reference :default "/Game/IA_Nest.IA_Nest")))

(event EventBeginPlay
  (CallFunction|SetupInput)
  (Variables|Default|SetFlaps (Variables|Default|GetFlapsMax)))

(event EventOnLanded
  (params (Hit :type Hit%20Result%20Structure%20%28by%20ref%29))
  (Variables|Default|SetOn%20Ground true))

(event EventTick
  (params (DeltaSeconds :type Float%20%28single-precision%29))
  (CallFunction|TickFlaps DeltaSeconds))

(fn ConstructionScript)

(fn TickFlaps
  (params (deltaTime :type Float%20%28double-precision%29))
  (if (> (+ deltaTime (Variables|Default|GetFlaps)) (Variables|Default|GetFlapsMax))
    (Variables|Default|SetFlaps 1.0)
    (else
      (Variables|Default|SetFlaps (+ deltaTime (Variables|Default|GetFlaps))))))

(fn Flap
  (bind _self self)
  (if (>= (Variables|Default|GetFlaps) (Variables|Default|GetFlapsMax))
    (Variables|Default|SetFlaps (- (Variables|Default|GetFlaps) 1.0))
    (Physics|AddImpulse (Variables|Character|GetCharacterMovement) (* (Variables|Default|GetImpulse%20Scalar) (Math|Vector|Normalize (+ (Transformation|GetActorUpVector _self) (Transformation|GetActorForwardVector _self)))) true)))

(fn Lift
  (Physics|AddForce (Variables|Character|GetCharacterMovement self) (* (* (Math|Vector|VectorLength (Math|Vector|ProjectVectorontoVector (Transformation|GetVelocity) (Transformation|GetActorForwardVector))) 5e+01) (Transformation|GetActorUpVector))))

(fn SetupInput)

(fn Pitch
  (params (Input%20Value :type Float%20%28double-precision%29))
  ;[1 1 1] Quaternion attempt
  (bind _returnvalue (Class|FlightQuaternion|EulertoQuaternion (Math|Rotator|MakeRotator 0.0 Input%20Value 0.0)))
  (Class|FlightQuaternion|AddActorLocalRotationQuat self _returnvalue))

(fn Roll
  (params (Input%20Value :type Float%20%28double-precision%29))
  ;[1 1 1] Quaternion
  (bind _returnvalue (Class|FlightQuaternion|EulertoQuaternion (Math|Rotator|MakeRotator Input%20Value 0.0 0.0)))
  (Class|FlightQuaternion|AddActorLocalRotationQuat self _returnvalue))

(fn Yaw
  (params (Input%20Value :type Float%20%28double-precision%29))
  ;[1 1 1] Quaternion
  (bind _returnvalue (Class|FlightQuaternion|EulertoQuaternion (Math|Rotator|MakeRotator 0.0 0.0 Input%20Value)))
  (Class|FlightQuaternion|AddActorLocalRotationQuat self _returnvalue))