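; BP_NestPrototype is a prototype nest actor that tracks Comfort and Durability and absorbs items that touch it.
; A one-second timer, looping if Durability starts positive, drains Durability by DegradationSpeed and prints "Game Over" once it is depleted.
; Overlapping AbstractItem actors add their comfort and durability values to the nest and are destroyed.
; Tick prints both stats on screen as keyed debug text.
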(event Custom|Nest%20Deteriorate
  (if (> (Variables|Default|GetDurability) 0.0)
    (Variables|Default|SetDurability (- (Variables|Default|GetDurability) (Variables|Default|GetDegradationSpeed)))
    (else
      (Development|PrintString "Game Over" true true "(R=1.000000,G=0.000000,B=0.028023,A=1.000000)"))))

(event EventBeginPlay
  (Utilities|Time|SetTimerbyEvent (delegate Custom|Nest%20Deteriorate) 1.0 (> (Variables|Default|GetDurability) 0.0)))

(event Collision|EventActorBeginOverlap
  (params (OtherActor :type Actor%20Object%20Reference))
  (bind _asabstract_item (Utilities|Casting|CastToAbstractItem OtherActor)
    (:then
      (Variables|Default|SetComfort (+ (Variables|Default|GetComfort) (Variables|/Script/BirdGame.AbstractItem|GetmyComfort _asabstract_item)))
      (Variables|Default|SetDurability (+ (Variables|Default|GetDurability) (Variables|/Script/BirdGame.AbstractItem|GetmyDurability _asabstract_item)))
      (Development|PrintString "Cast Succeed")
      (Actor|DestroyActor _asabstract_item))
    (:CastFailed
      (Development|PrintText "Cast Failed"))))

(event EventTick
  (params (DeltaSeconds :type Float%20%28single-precision%29))
  (Development|PrintText (Utilities|Text|ToText(Float) (Variables|Default|GetComfort) "HalfToEven" true) true true "(R=0.000000,G=0.660602,B=1.000000,A=1.000000)" 2.0 "Comfort")
  (Development|PrintText (Utilities|Text|ToText(Float) (Variables|Default|GetDurability) "HalfToEven" true) true true "(R=1.000000,G=0.728688,B=0.000000,A=1.000000)" 2.0 "Durability"))

(fn ConstructionScript)